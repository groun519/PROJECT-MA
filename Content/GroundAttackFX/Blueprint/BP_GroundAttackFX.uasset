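; BP_GroundAttackFX is an actor that repeatedly plays a configurable Niagara effect, named as a ground attack, at its placed position.
; BeginPlay enters a self-calling loop: a short random delay, a system spawn, a fixed wait, then the custom Again event restarts it.
; Each spawn uses the actor's location plus an offset variable and its rotation with yaw turned a quarter turn.
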(event `Again`
  (bind (_returnvalue_roll _returnvalue_pitch _returnvalue_yaw) (`KismetMathLibrary.BreakRotator` (`self.K2_GetActorRotation`)))
  (`KismetSystemLibrary.Delay` (`KismetMathLibrary.RandomFloatInRange` (`self.Delay`) 0.5) :!label _label)
  (`NiagaraFunctionLibrary.SpawnSystemAtLocation` (`self.Niagara System`) (+ (`self.K2_GetActorLocation`) (`self.add location`)) (`KismetMathLibrary.MakeRotator` _returnvalue_roll _returnvalue_pitch (+ _returnvalue_yaw 90.0)))
  (`KismetSystemLibrary.Delay` 4.0)
  (`self.Again`))

(event `self.ReceiveBeginPlay`
  (goto _label))

(fn `UserConstructionScript`)