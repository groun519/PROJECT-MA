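; Gameplay ability for a flinch hit reaction, activated from a gameplay event on an MACharacter avatar.
; As wired, activation only commits the ability and casts the avatar, without playing a montage or ending the ability.
; A disconnected branch would play the character's flinch montage from a section chosen from the event data, then print a debug string and end the ability on completion, blend out, interruption or cancellation.
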(event `self.K2_ActivateAbilityFromEvent`
  (params (EventData :type "GameplayEventData Structure (by ref)"))
  (`self.K2_CommitAbility`)
  (bind _asmacharacter (cast `MACharacter` (`self.GetAvatarActorFromActorInfo`))))